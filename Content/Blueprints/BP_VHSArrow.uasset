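; BP_VHSArrow is a VR indicator actor for the owning VRCharacter's Virtual Head Stick, shown while either trigger is held.
; Each tick it sits ahead of and below the camera, following its yaw, while the GenericHMD component copies the full camera rotation.
; The HMD component's relative X/Y offset reflects the stick's current values, scaled by data-table padding and clamped.
; Releasing both triggers hides the cylinder and HMD and recenters the latter.
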(event `self.ReceiveBeginPlay`
  (bind _asvrcharacter (cast `/Game/Blueprints/VRCharacter` (`self.GetOwner`)))
  (set `self.VRCharacter` _asvrcharacter))

(event `self.ReceiveTick`
  (params (DeltaSeconds :type "Float (single-precision)"))
  (`self.UpdatePositionAndRotation`))

(event `UpdatePositionAndRotation`
  (bind _vrcharacter (`self.VRCharacter`))
  (bind _vrcharacter_2 (`self.VRCharacter`))
  (bind _virtualheadstick (`/Game/Blueprints/VRCharacter.VirtualHeadStick` (`self.VRCharacter`)))
  (bind (_returnvalue_location _returnvalue_rotation) (`KismetMathLibrary.BreakTransform` (`SceneComponent.K2_GetComponentToWorld` (`/Game/Blueprints/VRCharacter.Camera` _vrcharacter_2))))
  (bind ((`PaddingX_24_5E5E729A480C9FCDE4506488DDDC059C` _paddingx) (`PaddingY_30_ED422D354846C681E16B2898E6D7A02C` _paddingy)) (break `/Game/DataTables/VHSDataTableStruct` (`/Game/Blueprints/VirtualHeadStick.VHSDataTable` _virtualheadstick)))
  (`/Engine/EditorBlueprintResources/StandardMacros.IsValid` _vrcharacter_2
    (:`Is Valid`
      (`|ExecutionSequence`
        (:`then_0`
          (`self.K2_SetActorLocationAndRotation` (+ _returnvalue_location (* (`KismetMathLibrary.GetForwardVector` _returnvalue_rotation) 50.0) (* (`KismetMathLibrary.GetUpVector` _returnvalue_rotation) -30.0)) (`KismetMathLibrary.MakeRotator` 0.0 0.0 (.yaw _returnvalue_rotation)))
          (`SceneComponent.K2_SetWorldRotation` (`self.GenericHMD`) _returnvalue_rotation false false))
        (:`then_1`
          (if (or (`/Game/Blueprints/VRCharacter.IsTriggerLeft?` _vrcharacter) (`/Game/Blueprints/VRCharacter.IsTriggerRight?` _vrcharacter))
            (`SceneComponent.SetVisibility` (`self.SM_FatCylinder`) true false)
            (`SceneComponent.SetVisibility` (`self.GenericHMD`) true false)
            (`SceneComponent.K2_SetRelativeLocation` (`self.GenericHMD`) (`KismetMathLibrary.MakeVector` (`KismetMathLibrary.FClamp` (* (/ 100.0 _paddingx) (`/Game/Blueprints/VirtualHeadStick.GetCurrentX` _virtualheadstick)) -50.0 100.0) (`KismetMathLibrary.FClamp` (* (/ 75.0 _paddingy) (`/Game/Blueprints/VirtualHeadStick.GetCurrentY` _virtualheadstick)) -75.0 75.0)) false false)
            (else
              (`SceneComponent.SetVisibility` (`self.SM_FatCylinder`) false false)
              (`SceneComponent.K2_SetRelativeLocation` (`self.GenericHMD`) (0.0 0.0 0.0) false false)
              (`SceneComponent.SetVisibility` (`self.GenericHMD`) false false))))))))

(fn `UserConstructionScript`)
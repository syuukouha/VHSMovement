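; Virtual head stick that turns head-tracking motion into planar movement and rotation values, like a joystick.
; Reset captures the origin, and Update tracks current and previous head position, up-vector stick tip and rotation.
; Weighted base and tip motion drives X/Y, while rotation change drives turning.
; Output requires motion away from center beyond padding and scales with speed between thresholds, all tuned by a data table row.
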(fn `GetCurrentX`
  (returns (ReturnValue :type "Float (double-precision)"))
  (bind _currentbase_x (`KismetMathLibrary.BreakVector` (`self.CurrentBase`)))
  (bind _currenttop_x (`KismetMathLibrary.BreakVector` (`self.CurrentTop`)))
  (bind (_sticklength _basex _basey _topx) (break `/Game/DataTables/VHSDataTableStruct` (`self.VHSDataTable`)))
  (return (+ (* _currentbase_x _basex) (* _currenttop_x _topx))))

(fn `GetCurrentY`
  (returns (ReturnValue :type "Float (double-precision)"))
  (bind (_currentbase_x _currentbase_y) (`KismetMathLibrary.BreakVector` (`self.CurrentBase`)))
  (bind (_currenttop_x _currenttop_y) (`KismetMathLibrary.BreakVector` (`self.CurrentTop`)))
  (bind (_sticklength _basex _basey _topx _topy) (break `/Game/DataTables/VHSDataTableStruct` (`self.VHSDataTable`)))
  (return (+ (* _currentbase_y _basey) (* _currenttop_y _topy))))

(fn `GetDeltaRotation`
  (returns (ReturnValue :type "Float (double-precision)"))
  (return (- (`self.CurrentRotation`) (`self.LastRotation`))))

(fn `GetDeltaX`
  (returns (ReturnValue :type "Float (double-precision)"))
  (bind (_sticklength _basex _basey _topx) (break `/Game/DataTables/VHSDataTableStruct` (`self.VHSDataTable`)))
  (bind _returnvalue_x (`KismetMathLibrary.BreakVector` (- (`self.CurrentTop`) (`self.LastTop`))))
  (bind _returnvalue_x_2 (`KismetMathLibrary.BreakVector` (- (`self.CurrentBase`) (`self.LastBase`))))
  (return (+ (* _returnvalue_x_2 _basex) (* _returnvalue_x _topx))))

(fn `GetDeltaY`
  (returns (ReturnValue :type "Float (double-precision)"))
  (bind (_sticklength _basex _basey _topx _topy) (break `/Game/DataTables/VHSDataTableStruct` (`self.VHSDataTable`)))
  (bind (_returnvalue_x _returnvalue_y) (`KismetMathLibrary.BreakVector` (- (`self.CurrentTop`) (`self.LastTop`))))
  (bind (_returnvalue_x_2 _returnvalue_y_2) (`KismetMathLibrary.BreakVector` (- (`self.CurrentBase`) (`self.LastBase`))))
  (return (+ (* _returnvalue_y_2 _basey) (* _returnvalue_y _topy))))

(fn `GetDirection`
  (params (Value :type "Float (double-precision)"))
  (returns (ReturnValue :type "Float (double-precision)"))
  (return (`KismetMathLibrary.SelectFloat` 1.0 -1.0 (> Value 0.0))))

(fn `GetRatio`
  (params (Value :type "Float (double-precision)") (Upper :type "Float (double-precision)") (Lower :type "Float (double-precision)"))
  (returns (ReturnValue :type "Float (double-precision)"))
  (if (> Value Upper)
    (return 1.0)
    (elif (> Value Lower)
      (return (/ (- Value Lower) (- Upper Lower)))
      (else
        (return 0.0)))))

(fn `GetValueMove`
  (returns (NewParam :type "Vector Structure"))
  (return (`KismetMathLibrary.MakeVector` (`self.GetValueX`) (`self.GetValueY`))))

(fn `GetValueRotation`
  (returns (ReturnValue :type "Float (double-precision)"))
  (bind ((`UpperRotation_34_2A70CDEA400DE9514616349C07B97B4C` _upperrotation) (`LowerRotation_40_714AB28F4027548FAE6021B157051C0B` _lowerrotation)) (break `/Game/DataTables/VHSDataTableStruct` (`self.VHSDataTable`)))
  (return (`KismetMathLibrary.SelectFloat` (* (`self.GetDirection` (`self.GetDeltaRotation`)) (`.SpeedRotation_23_75480FFB461C0C05CD3BE1A0D2AA2F27` (break `/Game/DataTables/VHSDataTableStruct` (`self.VHSDataTable`))) (`self.GetRatio` (/ (`KismetMathLibrary.Abs` (`self.GetDeltaRotation`)) (`self.DeltaSeconds`)) _upperrotation _lowerrotation) (`self.DeltaSeconds`)) 0.0 (and (> (* (`self.CurrentRotation`) (`self.GetDeltaRotation`)) 0.0) (> (`KismetMathLibrary.Abs` (`self.CurrentRotation`)) (`.PaddingRotation_31_7A259038436B5D22A003BD885696CD4D` (break `/Game/DataTables/VHSDataTableStruct` (`self.VHSDataTable`))))))))

(fn `GetValueX`
  (returns (ReturnValue :type "Float (double-precision)"))
  (locals (CurrentSpeedX :type "Float (double-precision)"))
  (bind _returnvalue (`self.GetCurrentX`))
  (bind ((`UpperX_32_8E2D13A6492EDF92CF698497AC31C43B` _upperx) (`LowerX_38_694432B148F841B6982CBA8C5A79C050` _lowerx)) (break `/Game/DataTables/VHSDataTableStruct` (`self.VHSDataTable`)))
  (set `local.CurrentSpeedX` (`.SpeedX_18_11E5B6F2477F4866F5BC439D9F6BECFB` (break `/Game/DataTables/VHSDataTableStruct` (`self.VHSDataTable`))))
  (return (`KismetMathLibrary.SelectFloat` (* (`self.GetDirection` (`self.GetDeltaX`)) (`local.CurrentSpeedX`) (`self.GetRatio` (/ (`KismetMathLibrary.Abs` (`self.GetDeltaX`)) (`self.DeltaSeconds`)) _upperx _lowerx) (`self.DeltaSeconds`)) 0.0 (and (> (* _returnvalue (`self.GetDeltaX`)) 0.0) (> (`KismetMathLibrary.Abs` _returnvalue) (`.PaddingX_24_5E5E729A480C9FCDE4506488DDDC059C` (break `/Game/DataTables/VHSDataTableStruct` (`self.VHSDataTable`))))))))

(fn `GetValueY`
  (returns (ReturnValue :type "Float (double-precision)"))
  (bind ((`UpperY_33_D93E066D47588E914DCCC495283892FD` _uppery) (`LowerY_39_685A17B044C51B43867F4686B2EA284A` _lowery)) (break `/Game/DataTables/VHSDataTableStruct` (`self.VHSDataTable`)))
  (return (`KismetMathLibrary.SelectFloat` (* (`self.GetDirection` (`self.GetDeltaY`)) (`.SpeedY_22_F41B602C4DBCFEFB505A03B7E8841E17` (break `/Game/DataTables/VHSDataTableStruct` (`self.VHSDataTable`))) (`self.GetRatio` (/ (`KismetMathLibrary.Abs` (`self.GetDeltaY`)) (`self.DeltaSeconds`)) _uppery _lowery) (`self.DeltaSeconds`)) 0.0 (and (> (* (`self.GetCurrentY`) (`self.GetDeltaY`)) 0.0) (> (`KismetMathLibrary.Abs` (`self.GetCurrentY`)) (`.PaddingY_30_ED422D354846C681E16B2898E6D7A02C` (break `/Game/DataTables/VHSDataTableStruct` (`self.VHSDataTable`))))))))

(fn `Initialize`
  (bind _returnvalue (`|GetDataTableRow` "/Game/DataTables/VHSDataTable.VHSDataTable" "Default")
    (:`then`
      (set `self.VHSDataTable` _returnvalue))))

(fn `Reset`
  (params (HeadTransform :type "/Game/Blueprints/HeadTransform Object Reference"))
  (set `self.DeltaSeconds` 1.0)
  (set `self.OriginBase` (`self.GetAbsoluteBase` HeadTransform))
  (set `self.OriginRotation` (`self.GetAbsoluteRotation` HeadTransform))
  (bind _output_get (set `self.LastBase` (`self.GetRelativeTop` HeadTransform)))
  (set `self.CurrentBase` _output_get)
  (bind _output_get_2 (set `self.LastTop` (`self.GetRelativeTop` HeadTransform)))
  (set `self.CurrentTop` _output_get_2)
  (bind _output_get_3 (set `self.LastRotation` (`self.GetRelativeRotation` HeadTransform)))
  (set `self.CurrentRotation` _output_get_3))

(fn `Update`
  (params (HeadTransform :type "/Game/Blueprints/HeadTransform Object Reference") (DeltaSeconds :type "Float (double-precision)"))
  (set `self.DeltaSeconds` DeltaSeconds)
  (set `self.LastBase` (`self.CurrentBase`))
  (set `self.LastTop` (`self.CurrentTop`))
  (set `self.LastRotation` (`self.CurrentRotation`))
  (set `self.CurrentBase` (`self.GetRelativeBase` HeadTransform))
  (set `self.CurrentTop` (`self.GetRelativeTop` HeadTransform))
  (set `self.CurrentRotation` (`self.GetRelativeRotation` HeadTransform)))